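; BP_OSCServer is an actor that drives a chamfer cube mesh from ArUco marker tracking data.
; BeginPlay sets the CG221ArucoMarker component's UDP port; on each Tick with the new-data flag set, it prints position, angles and timestamp milliseconds.
; The position is applied as an additive local offset, so movement accumulates.
; An unconnected SetWorldTransform node would apply absolute position and rotation instead.
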(event `self.ReceiveBeginPlay`
  (set `CG221ArucoMarkerComponent.UdpPort` 5005 (`self.CG221ArucoMarker`)))

(event `self.ReceiveTick`
  (params (DeltaSeconds :type "Float (single-precision)"))
  (bind _cg221arucomarker (`self.CG221ArucoMarker`))
  (bind (_posx _posy _posz _angx _angy _angz _timestamp) (break `ArucoMarker` (`CG221ArucoMarkerComponent.ArucoMarkerData` _cg221arucomarker)))
  (if (`CG221ArucoMarkerComponent.bNewDataFlag` _cg221arucomarker)
    (`KismetSystemLibrary.PrintString` (`KismetTextLibrary.Conv_TextToString` (`|FormatText` "ArucoMarker Data {0} {1} {2} {3} {4} {5} {6}" _posx _posy _posz _angx _angy _angz (`.Millisecond` (`KismetMathLibrary.BreakDateTime` _timestamp)))) true true (struct :`R` 1.0 :`B` 0.142179 :`A` 1.0) 0.0)
    (`SceneComponent.K2_AddLocalOffset` (`self.SM_ChamferCube`) (`KismetMathLibrary.MakeVector` _posx _posy _posz) false false)))

(fn `UserConstructionScript`)